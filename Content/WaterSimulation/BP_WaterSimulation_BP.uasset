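; Water surface actor that simulates interactive ripples on a plane using render targets and materials.
; A player-following scene capture renders the pawn and moving actors inside the capture volume, and a compute material draws that capture into the current heightfield.
; A fixed-step loop cycles three height targets, feeding the previous two into the wave simulation material.
; A normal pass follows, and height and normal textures drive the water surface material.
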(event OnComponentBeginOverlap(SimulationCaptureVolume)
  (params (OverlappedComponent :type Primitive%20Component%20Object%20Reference) (OtherActor :type Actor%20Object%20Reference) (OtherComp :type Primitive%20Component%20Object%20Reference) (OtherBodyIndex :type Integer) (bFromSweep :type Boolean) (SweepResult :type Hit%20Result%20Structure%20%28by%20ref%29))
  ;[0.15 0.15 0.15 0.5] Simulation Capture Overlap Event
  (Utilities|Array|AddUnique (Variables|Default|GetCaptureActor) OtherActor)
  (Rendering|SceneCapture|ShowOnlyActorComponents (Variables|Default|GetSceneCaptureComponent2D) OtherActor false))

(event OnComponentEndOverlap(SimulationCaptureVolume)
  (params (OverlappedComponent :type Primitive%20Component%20Object%20Reference) (OtherActor :type Actor%20Object%20Reference) (OtherComp :type Primitive%20Component%20Object%20Reference) (OtherBodyIndex :type Integer))
  ;[0.15 0.15 0.15 0.5] Simulation Capture Overlap Event
  (if (Utilities|Array|ContainsItem (Variables|Default|GetCaptureActor) OtherActor)
    (Utilities|Array|RemoveItem (Variables|Default|GetCaptureActor) OtherActor)
    (Class|SceneCaptureComponent|RemoveShowOnlyActorComponents (Variables|Default|GetSceneCaptureComponent2D) OtherActor false)))

(event EventBeginPlay
  (bind _scenecapturecomponent2d (Variables|Default|GetSceneCaptureComponent2D))
  (bind _plane (Variables|Default|GetPlane))
  (bind _textureresolution (Variables|WaterSimulation|Setting|GetTextureResolution))
  (bind _textureresolution_2 (Variables|WaterSimulation|Setting|GetTextureResolution))
  (bind _capturetextureresolution (Variables|WaterSimulation|Setting|GetCaptureTextureResolution))
  (bind _textureresolution_3 (Variables|WaterSimulation|Setting|GetTextureResolution))
  (bind _textureresolution_4 (Variables|WaterSimulation|Setting|GetTextureResolution))
  (bind _returnvalue (Transformation|GetWorldScale _plane))
  (Utilities|FlowControl|Sequence
    (:then_0
      (bind _returnvalue_2 (Rendering|CreateRenderTarget2D _capturetextureresolution _capturetextureresolution "RTF_R8"))
      (Variables|WaterSimulation|Texture|SetRT_Capture _returnvalue_2)
      (bind _returnvalue_3 (Rendering|CreateRenderTarget2D _textureresolution _textureresolution "RTF_R16f"))
      (Variables|WaterSimulation|Texture|SetRT_Height_0 _returnvalue_3)
      (bind _returnvalue_4 (Rendering|CreateRenderTarget2D _textureresolution_3 _textureresolution_3 "RTF_R16f"))
      (Variables|WaterSimulation|Texture|SetRT_Height_2 _returnvalue_4)
      (bind _returnvalue_5 (Rendering|CreateRenderTarget2D _textureresolution_2 _textureresolution_2 "RTF_R16f"))
      (Variables|WaterSimulation|Texture|SetRT_Height_1 _returnvalue_5)
      (bind _returnvalue_6 (Rendering|CreateRenderTarget2D _textureresolution_4 _textureresolution_4 "RTF_RGBA16f"))
      (Variables|WaterSimulation|Texture|SetRT_HeightNormal _returnvalue_6)
      ;[0.15 0.15 0.15 0.5] 初始化清除RT纹理
      (Rendering|ClearRenderTarget2D (Variables|WaterSimulation|Texture|GetRT_Capture))
      (Rendering|ClearRenderTarget2D (Variables|WaterSimulation|Texture|GetRT_Height_0))
      (Rendering|ClearRenderTarget2D (Variables|WaterSimulation|Texture|GetRT_Height_2))
      (Rendering|ClearRenderTarget2D (Variables|WaterSimulation|Texture|GetRT_Height_1))
      (Rendering|ClearRenderTarget2D (Variables|WaterSimulation|Texture|GetRT_HeightNormal)))
    (:then_1
      (Variables|/Script/Engine.SceneCaptureComponent2D|SetTextureTarget _scenecapturecomponent2d (Variables|WaterSimulation|Texture|GetRT_Capture))
      (Rendering|SceneCapture|ShowOnlyActorComponents _scenecapturecomponent2d (Game|Player|GetPlayerPawn 0) false)
      (Variables|Default|SetPlane%20Scale (Math|Float|Max(Float) (.x _returnvalue) (.y _returnvalue)))
      ;[0.15 0.15 0.15 0.5] Initialize Simulation Capture Actor
      (Utilities|FlowControl|Delay 0.1)
      (bind _output_get (Variables|Default|SetOverlapping%20Actors (Collision|GetOverlappingActors (Variables|Default|GetSimulationCaptureVolume) 0 :!class /Script/Engine.PrimitiveComponent)))
      (for _array_element _output_get
        (Utilities|Array|AddUnique (Variables|Default|GetCaptureActor) _array_element)
        (Rendering|SceneCapture|ShowOnlyActorComponents (Variables|Default|GetSceneCaptureComponent2D) _array_element false)))
    (:then_2
      (Rendering|Material|SetScalarParameterValue (Variables|Default|GetMID_WaterSurface) "Canvas Size" (Variables|Default|GetPlane%20Scale) :!class /Script/Engine.MaterialInstanceDynamic)
      (bind _returnvalue_7 (Rendering|Material|CreateDynamicMaterialInstance (Variables|WaterSimulation|Materials|GetM_WaveCompute) "None" "None" :!class /Script/Engine.KismetMaterialLibrary))
      (bind _output_get_2 (Variables|Default|SetMID_WaveCompute _returnvalue_7))
      (Rendering|Material|SetVectorParameterValue _output_get_2 "Plane Location" (Math|Conversions|ToLinearColor(Vector) (Transformation|GetWorldLocation (Variables|Default|GetDefaultSceneRoot))) :!class /Script/Engine.MaterialInstanceDynamic)
      (Rendering|Material|SetScalarParameterValue (Variables|Default|GetMID_WaveCompute) "Texture Resolution" (Math|Conversions|ToFloat(Integer) (Variables|WaterSimulation|Setting|GetTextureResolution)) :!class /Script/Engine.MaterialInstanceDynamic)
      (Rendering|Material|SetScalarParameterValue (Variables|Default|GetMID_WaveCompute) "Canvas Size" (Variables|Default|GetPlane%20Scale) :!class /Script/Engine.MaterialInstanceDynamic)
      (bind _returnvalue_8 (Rendering|Material|CreateDynamicMaterialInstance (Variables|WaterSimulation|Materials|GetM_WaveSimulation) "None" "None" :!class /Script/Engine.KismetMaterialLibrary))
      (bind _output_get_3 (Variables|Default|SetMID_WaveSimulation _returnvalue_8))
      (Rendering|Material|SetScalarParameterValue _output_get_3 "Canvas Size" (Variables|Default|GetPlane%20Scale) :!class /Script/Engine.MaterialInstanceDynamic)
      ;[0.15 0.15 0.15 0.5] 初始化wavenormal
      (bind _returnvalue_9 (Rendering|Material|CreateDynamicMaterialInstance (Variables|WaterSimulation|Materials|GetM_WaveNormal) "None" "None" :!class /Script/Engine.KismetMaterialLibrary))
      (bind _output_get_4 (Variables|Default|SetMID_WaveNormal _returnvalue_9))
      (Rendering|Material|SetScalarParameterValue _output_get_4 "Canvas Size" (Variables|Default|GetPlane%20Scale) :!class /Script/Engine.MaterialInstanceDynamic))))

(event EventTick
  (params (DeltaSeconds :type Float%20%28single-precision%29))
  (bind _returnvalue (Game|Player|GetPlayerPawn 0))
  (bind _simulationspeed (Variables|WaterSimulation|Setting|GetSimulationSpeed))
  (bind _scenecapturecomponent2d (Variables|Default|GetSceneCaptureComponent2D))
  (bind _scenecapturecomponent2d_2 (Variables|Default|GetSceneCaptureComponent2D))
  (bind _returnvalue_2 (Transformation|GetActorLocation _returnvalue))
  (bind _returnvalue_3 (Math|Float|Min(Float) _simulationspeed 1.2e+02))
  (bind _returnvalue_4 (/ 1.0 _returnvalue_3))
  (Variables|Default|SetDelta%20Seconds DeltaSeconds)
  (Utilities|FlowControl|Sequence
    (:then_0
      (Rendering|Material|SetTextureParameterValue (Variables|Default|GetMID_WaveCompute) "Capture" (Variables|WaterSimulation|Texture|GetRT_Capture))
      (Rendering|Material|SetVectorParameterValue (Variables|Default|GetMID_WaveCompute) "Capture Location" (Math|Conversions|ToLinearColor(Vector) (Transformation|GetActorLocation (Game|Player|GetPlayerPawn 0))) :!class /Script/Engine.MaterialInstanceDynamic)
      (bind _rt_height (CallFunction|GetRenderTargetTexture (Variables|Default|GetHeightindex)))
      (Rendering|DrawMaterialtoRenderTarget _rt_height (Variables|Default|GetMID_WaveCompute))
      (Variables|Default|SetFrameRate (+ (Variables|Default|GetFrameRate) (Variables|Default|GetDelta%20Seconds)))
      (while (> (Variables|Default|GetFrameRate) _returnvalue_4)
        (Variables|Default|SetFrameRate (- (Variables|Default|GetFrameRate) _returnvalue_4))
        (Variables|Default|SetHeightindex (Math|Integer|%(Integer) (+ (Variables|Default|GetHeightindex) 1) 3))
        (bind _rt_height_2 (CallFunction|GetLastRenderTargetTexture (Variables|Default|GetHeightindex) 1))
        (Rendering|Material|SetTextureParameterValue (Variables|Default|GetMID_WaveSimulation) "Previous Height1" _rt_height_2)
        (bind _rt_height_3 (CallFunction|GetLastRenderTargetTexture (Variables|Default|GetHeightindex) 2))
        (Rendering|Material|SetTextureParameterValue (Variables|Default|GetMID_WaveSimulation) "Previous Height2" _rt_height_3)
        (bind _rt_height_4 (CallFunction|GetRenderTargetTexture (Variables|Default|GetHeightindex)))
        (bind (_canvas _size _context) (Rendering|BeginDrawCanvastoRenderTarget _rt_height_4))
        (Canvas|DrawMaterial :self _canvas :RenderMaterial (Variables|Default|GetMID_WaveSimulation) :ScreenSize _size :CoordinateSize "(X=1.000000,Y=1.000000)" :PivotPoint "(X=0.500000,Y=0.500000)")
        (Rendering|EndDrawCanvastoRenderTarget _context)
        (bind _rt_height_5 (CallFunction|GetRenderTargetTexture (Variables|Default|GetHeightindex)))
        (Rendering|Material|SetTextureParameterValue (Variables|Default|GetMID_WaterSurface) "Heightfield" _rt_height_5))
      ;[0.15 0.15 0.15 0.5] WaveNormal
      (bind _rt_height_6 (CallFunction|GetRenderTargetTexture (Variables|Default|GetHeightindex)))
      (Rendering|Material|SetTextureParameterValue (Variables|Default|GetMID_WaveNormal) "Heightfield Height" _rt_height_6)
      (Rendering|DrawMaterialtoRenderTarget (Variables|WaterSimulation|Texture|GetRT_HeightNormal) (Variables|Default|GetMID_WaveNormal))
      (Rendering|Material|SetTextureParameterValue (Variables|Default|GetMID_WaterSurface) "Heightfield Normal" (Variables|WaterSimulation|Texture|GetRT_HeightNormal)))
    (:then_1
      (Transformation|SetWorldLocation _scenecapturecomponent2d (Math|Vector|MakeVector (.x _returnvalue_2) (.y _returnvalue_2) (.z (Transformation|GetWorldLocation _scenecapturecomponent2d))) false false)
      (for _array_element (Variables|Default|GetCaptureActor)
        (if (> (Math|Vector|VectorLength (Transformation|GetVelocity _array_element)) 1e+02)
          (Rendering|SceneCapture|ShowOnlyActorComponents _scenecapturecomponent2d_2 _array_element false)
          (else
            (Class|SceneCaptureComponent|RemoveShowOnlyActorComponents _scenecapturecomponent2d_2 _array_element false)))))))

(fn ConstructionScript
  (bind _scenecapturecomponent2d (Variables|Default|GetSceneCaptureComponent2D))
  (bind _returnvalue (Rendering|Material|CreateDynamicMaterialInstance (Variables|Default|GetPlane) 0 (Variables|WaterSimulation|Materials|GetM_WaterSurface) "None" :!class /Script/Engine.PrimitiveComponent))
  (bind _output_get (Variables|Default|SetMID_WaterSurface _returnvalue))
  (Rendering|Material|SetMaterial (Variables|Default|GetPlane) 0 _output_get)
  (Transformation|SetWorldRotation _scenecapturecomponent2d "-90.000000,-90.000000,0.000000" false false)
  (Transformation|SetWorldScale3D _scenecapturecomponent2d "0, 0, 0"))

(fn GetRenderTargetTexture
  (params (index :type Integer))
  (if (== index 0)
    (return (Variables|WaterSimulation|Texture|GetRT_Height_0))
    (elif (== index 1)
      (return (Variables|WaterSimulation|Texture|GetRT_Height_1))
      (else
        (return (Variables|WaterSimulation|Texture|GetRT_Height_2))))))

(fn GetLastRenderTargetTexture
  (params (Current%20Height%20index :type Integer) (Nums%20Frame%20Old%20index :type Integer))
  (bind _rt_height (CallFunction|GetRenderTargetTexture (Math|Integer|%(Integer) (+ (- Current%20Height%20index Nums%20Frame%20Old%20index) 3) 3)))
  (return _rt_height))